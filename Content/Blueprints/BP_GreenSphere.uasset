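; BP_GreenSphere is an interactive sphere that changes color through focus, blur and activate interface events.
; It swaps the sphere's material to red on focus, green on blur and blue on activation.
; Activation also prints the result of GetNextValidIndex, which increments a wrapping skybox index.
; The skybox hookup is unfinished: the overlap handler only self-assigns its reference, the ChangeMaterialMessage call is disconnected, and ChangeMaterial is a stub.
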(event `/Game/Blueprints/BPI_Interaction.OnFocus`
  ;[1 1 1] Green Sphere Interface Implementations
  (`PrimitiveComponent.SetMaterial` (`self.Sphere`) 0 "/Game/Materials/M_Red.M_Red"))

(event `/Game/Blueprints/BPI_Interaction.OnBlur`
  ;[1 1 1] Green Sphere Interface Implementations
  (`PrimitiveComponent.SetMaterial` (`self.Sphere`) 0 "/Game/Materials/M_Green.M_Green"))

(event `/Game/Blueprints/BPI_Interaction.OnActivate`
  ;[1 1 1] Green Sphere Interface Implementations
  (`PrimitiveComponent.SetMaterial` (`self.Sphere`) 0 "/Game/Materials/M_Blue.M_Blue")
  (bind _outputindex (`self.GetNextValidIndex`))
  (`KismetSystemLibrary.PrintString` (`KismetStringLibrary.Conv_IntToString` _outputindex)))

(event `self.BPSkybox1_Ref.OnActorBeginOverlap`
  (params (OverlappedActor :type "Actor Object Reference") (OtherActor :type "Actor Object Reference"))
  ;[1 1 1] Green Sphere Interface Implementations
  (bind _output_get (set `self.BPSkybox1_Ref` (`self.BPSkybox1_Ref`))))

(fn `ChangeMaterial`
  (params (IndexInt :type Integer :default 0))
  (returns (ReturnString :type String))
  (return ""))

(fn `GetNextValidIndex`
  (returns (OutputIndex :type Integer))
  (bind _result (`/Engine/EditorBlueprintResources/StandardMacros.IncrementInt` (`self.SkyboxIndex`))
    (:`  `
      (if (<= _result 3)
        (return _result)
        (else
          (bind _output_get (set `self.SkyboxIndex` (`self.ZeroIndex`)))
          (return _output_get))))))

(fn `UserConstructionScript`
  (locals (MaterialName :type "MaterialInstanceDynamic Object Reference"))
  ;[1 1 1] Create Dynamic Material Instance
)