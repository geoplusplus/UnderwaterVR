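; Skybox actor for an underwater VR project that applies skybox materials to its SkySphere mesh.
; The construction script creates a dynamic instance of M_Skybox1 and prints a welcome message.
; ChangeMaterial switches skybox materials by index, also using that index as the material slot.
; Index 1 sets plain M_Skybox1 without reaching the string return, and the M_Skybox2 node is unconnected.
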(fn `ChangeMaterial`
  (params (IndexInt :type Integer))
  (returns (ReturnStr :type String))
  (switch `int` IndexInt
    (:`0`
      (`PrimitiveComponent.CreateDynamicMaterialInstance` (`self.SkySphere`) IndexInt "/Game/Materials/M_Skybox1.M_Skybox1")
      (return (`|GetArrayItem` (`self.StringArray`))))
    (:`1`
      (`PrimitiveComponent.SetMaterial` (`self.SkySphere`) IndexInt "/Game/Materials/M_Skybox1.M_Skybox1"))
    (:`2`
      (`PrimitiveComponent.CreateDynamicMaterialInstance` (`self.SkySphere`) IndexInt "/Game/Materials/M_Skybox3.M_Skybox3")
      (return (`|GetArrayItem` (`self.StringArray`))))
    (:`3`
      (`PrimitiveComponent.CreateDynamicMaterialInstance` (`self.SkySphere`) IndexInt "/Game/Materials/M_Skybox4.M_Skybox4")
      (return (`|GetArrayItem` (`self.StringArray`))))))

(fn `UserConstructionScript`
  (`PrimitiveComponent.CreateDynamicMaterialInstance` (`self.SkySphere`) (`self.IntIndex`) "/Game/Materials/M_Skybox1.M_Skybox1")
  (`KismetSystemLibrary.PrintString` "Welcome to Underwater VR" true true (struct :`R` 1.0 :`G` 1.0 :`B` 1.0 :`A` 1.0)))